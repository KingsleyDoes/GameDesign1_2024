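; BP_PotionIngredient is a collectible potion ingredient that the player gathers by walking into it.
; Overlapping PickupTrigger casts to BP_ThirdPersonCharacterCustom, increments its IngredientCount, prints the new total and destroys the ingredient.
; Pickup, Drop and PrimaryAction are empty; disconnected nodes retain unused held-item logic for hand attachment, physics dropping and consumption on a Can component.
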(event `/Game/Blueprints/BPI_Item.Pickup`
  (params (ParentMesh :type "SkeletalMeshComponent Object Reference")))

(event `/Game/Blueprints/BPI_Item.Drop`)

(event `/Game/Blueprints/BPI_Item.PrimaryAction`
  (params (ref_thirdPersonCharCustom :type "/Game/Blueprints/BP_ThirdPersonCharacterCustom Object Reference"))
  ;[1 1 1] Comment
)

(event `self.PickupTrigger.OnComponentBeginOverlap`
  (params (OverlappedComponent :type "PrimitiveComponent Object Reference") (OtherActor :type "Actor Object Reference") (OtherComp :type "PrimitiveComponent Object Reference") (OtherBodyIndex :type Integer) (bFromSweep :type Boolean) (SweepResult :type "HitResult Structure (by ref)"))
  (bind _asbp_third_person_character_custom (cast `/Game/Blueprints/BP_ThirdPersonCharacterCustom` OtherActor))
  (bind _ingredientcount (`/Game/Blueprints/BP_ThirdPersonCharacterCustom.IngredientCount` _asbp_third_person_character_custom))
  (set `/Game/Blueprints/BP_ThirdPersonCharacterCustom.IngredientCount` (+ _ingredientcount 1) _asbp_third_person_character_custom)
  (`KismetSystemLibrary.PrintString` (`KismetStringLibrary.Concat_StrStr` "You have " (`KismetStringLibrary.Conv_IntToString` _ingredientcount) " ingredient(s)"))
  (`self.K2_DestroyActor`))

(fn `UserConstructionScript`)